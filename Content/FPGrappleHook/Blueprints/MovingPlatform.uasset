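; Moving platform Blueprint that shuttles its static mesh back and forth between its starting position and an offset position.
; The construction script records the mesh's world location, adds MovementOffset, and makes that the first target.
; From BeginPlay, a self-calling Move event runs MoveComponentTo, pauses for StopTime, then uses a FlipFlop to swap targets.
; The stored world locations are passed as relative-location targets.
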(event `self.ReceiveBeginPlay`
  ;[0 0 0] Move event on begin
  (`self.Move`))

(event `Move`
  ;[0 0 0] Move to initial/offset location
  (`KismetSystemLibrary.MoveComponentTo` (`self.StaticMesh`) (`self.TargetLocation`) (struct) false false (`self.MoveTime`))
  (`KismetSystemLibrary.Delay` (`self.StopTime`))
  (`/Engine/EditorBlueprintResources/StandardMacros.FlipFlop`
    (:`A`
      (set `self.TargetLocation` (`self.InitialLocation`)))
    (:`B`
      (set `self.TargetLocation` (`self.OffsetLocation`))))
  (`self.Move`))

(fn `UserConstructionScript`
  (bind _returnvalue (`SceneComponent.K2_GetComponentLocation` (`self.StaticMesh`)))
  ;[0 0 0] Set offset location
  (set `self.InitialLocation` _returnvalue)
  (bind _output_get (set `self.OffsetLocation` (+ _returnvalue (`self.MovementOffset`))))
  (set `self.TargetLocation` _output_get))