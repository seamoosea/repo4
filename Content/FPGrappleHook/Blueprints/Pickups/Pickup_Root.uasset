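; Base grapple hook pickup actor that hands its hook class to the first-person character on overlap.
; Sphere overlap sets the character's HookClass only while HookState is false, then plays a throw sound and refreshes the grapple HUD stats.
; The construction script applies the configurable mesh and light color and caches the initial location.
; A bob-and-spin timeline exists but is never triggered.
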(event `self.Sphere.OnComponentBeginOverlap`
  (params (OverlappedComponent :type "PrimitiveComponent Object Reference") (OtherActor :type "Actor Object Reference") (OtherComp :type "PrimitiveComponent Object Reference") (OtherBodyIndex :type Integer) (bFromSweep :type Boolean) (SweepResult :type "HitResult Structure (by ref)"))
  ;[0 0 0] Overlap Event
  (bind _asfirst_person_character (cast `/Game/FPGrappleHook/FirstPersonBP/Blueprints/FirstPersonCharacter` OtherActor))
  (if (not (`/Game/FPGrappleHook/FirstPersonBP/Blueprints/FirstPersonCharacter.HookState` _asfirst_person_character))
    (set `/Game/FPGrappleHook/FirstPersonBP/Blueprints/FirstPersonCharacter.HookClass` (`self.HookClass`) _asfirst_person_character)
    (`GameplayStatics.PlaySound2D` "/Game/FPGrappleHook/Sounds/Wav/RopeThrow2.RopeThrow2")
    (`/Game/FPGrappleHook/Blueprints/Widget/GrappleHUD.UpdateGrappleStatsText` (`/Game/FPGrappleHook/FirstPersonBP/Blueprints/FirstPersonCharacter.GrappleHUD` _asfirst_person_character))))

(fn `UserConstructionScript`
  ;[0 0 0] Set pickup mesh and light color
  (`StaticMeshComponent.SetStaticMesh` (`self.StaticMesh`) (`self.PickupMesh`))
  (`LightComponent.SetLightColor` (`self.PointLight`) (`self.PickupColor`) true)
  (set `self.InitialLocation` (`self.K2_GetActorLocation`)))