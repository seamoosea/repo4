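; TutorialStand is a prop Blueprint for a tutorial stand in the FPGrappleHook content, with a configurable surface look.
; Its Construction Script creates a dynamic material instance on the second material slot of its static mesh and stores it.
; It then applies the Color, Metallic and Roughness variables as parameters on that instance.
; The event graph holds only disabled placeholder events, so it has no runtime logic.
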(fn `UserConstructionScript`
  ;[0 0 0] Set material paramaters of tutorial stand
  (bind _returnvalue (`PrimitiveComponent.CreateDynamicMaterialInstance` (`self.StaticMesh`) 1 null))
  (bind _output_get (set `self.StandMaterialInstance` _returnvalue))
  (`MaterialInstanceDynamic.SetVectorParameterValue` _output_get "Color" (`self.Color`))
  (`MaterialInstanceDynamic.SetScalarParameterValue` (`self.StandMaterialInstance`) "Metallic" (`self.Metallic`))
  (`MaterialInstanceDynamic.SetScalarParameterValue` (`self.StandMaterialInstance`) "Roughness" (`self.Roughness`)))