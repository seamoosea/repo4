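; Base grappling hook actor that flies toward its attach point, spinning and playing a randomly pitched rope-throw sound on spawn.
; Construction sets the mesh, projectile speeds from ThrowSpeed and a random spin direction.
; Tick spins the mesh until CloseRotateGate is called and, while Active, lerps the actor toward HookEndTrace plus MovingActorOffset.
; Interp speed rises as the socket-to-target distance shrinks relative to ThrowDistance.
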(event `self.ReceiveBeginPlay`
  ;[0 0 0] Rope throw sound
  (`GameplayStatics.PlaySoundAtLocation` (`self.RopeThrowSound`) (.location (`self.GetTransform`)) (.rotation (`self.GetTransform`)) 1.0 (`KismetMathLibrary.RandomFloatInRange` 0.5 1.5) 0.0 "/Game/FPGrappleHook/Sounds/Audio/DefaultAttenuation.DefaultAttenuation"))

(event `RotateHook`
  ;[0 0 0] Rotate hook
  (`/Engine/EditorBlueprintResources/StandardMacros.Gate` false :!label _label
    (:`Exit`
      (`SceneComponent.K2_AddLocalRotation` (`self.StaticMesh`) (* (`KismetMathLibrary.MakeRotator` 0.0 0.0 (`self.SpinSpeed`)) (`self.RotationDirection`)) false false))))

(event `CloseRotateGate`
  ;[0 0 0] Rotate hook
  (goto _label :!via `Close`))

(event `self.ReceiveTick`
  (params (DeltaSeconds :type "Float (single-precision)"))
  ;[0 0 0] Tick events
  (`self.RotateHook`)
  (`self.InterpToPoint`))

(event `InterpToPoint`
  ;[0 0 0] Interp to point event
  (if (`self.Active`)
    (`self.K2_SetActorLocationAndRotation` (`KismetMathLibrary.VLerp` (`self.K2_GetActorLocation`) (+ (`self.HookEndTrace`) (`self.MovingActorOffset`)) (`KismetMathLibrary.FInterpTo` 0.0 1.0 (`GameplayStatics.GetWorldDeltaSeconds`) (* (`self.ThrowSpeed`) (+ 1.0 (- 1.0 (/ (`KismetMathLibrary.VSize` (- (`self.HookSocketLocation`) (`self.HookEndTrace`))) (`self.ThrowDistance`))))))) (`self.K2_GetActorRotation`))))

(fn `UserConstructionScript`
  (bind _projectilemovement (`self.ProjectileMovement`))
  (bind _throwspeed (`self.ThrowSpeed`))
  (set `ProjectileMovementComponent.InitialSpeed` _throwspeed _projectilemovement)
  (set `ProjectileMovementComponent.MaxSpeed` _throwspeed _projectilemovement)
  (`StaticMeshComponent.SetStaticMesh` (`self.StaticMesh`) (`self.HookMesh`))
  (`|MultiGate` true
    (:`Out 0`
      (set `self.RotationDirection` 1.0))
    (:`Out 1`
      (set `self.RotationDirection` -1.0))))